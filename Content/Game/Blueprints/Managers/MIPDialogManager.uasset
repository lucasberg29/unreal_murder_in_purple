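; MIPDialogManager manages NPC dialog, providing a list of question choices for the current conversation.
; StartDialog stores the NPC's Id when no dialog is active, then TraverseTree picks an act function by CurrentLevel, with only Act1 wired.
; Act1 fills CurrentQuestions with hardcoded lines, read back through GetQuestions.
; AdvanceDialog and UpdateGameState are empty stubs, and nothing here clears IsInDialog.
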(fn `Act1`
  (switch `int` (`self.currentNPC`)
    (:`1`
      (`self.Questions` (`|MakeArray` "Why is the road blocked?" "News?" "Bye.")))))

(fn `AdvanceDialog`
  (params (choiceId :type Integer)))

(fn `GetQuestions`
  (returns (Questions :type "Array of String"))
  (return (`self.currentQuestions`)))

(fn `Questions`
  (params (Questions :type "Array of String"))
  (set `self.currentQuestions` Questions))

(fn `StartDialog`
  (params (NPC :type "/Game/Game/Blueprints/Characters/NPCs/InteractableNPC Object Reference"))
  (if (not (`self.isInDialog`))
    (set `self.currentNPC` (`/Game/Game/Blueprints/Interactables/Interactable.id` NPC))
    (`self.TraverseTree`)
    (set `self.isInDialog` true)))

(fn `TraverseTree`
  (switch `int` (`self.currentLevel`)
    (:`1`
      (`self.Act1`))))

(fn `UpdateGameState`)